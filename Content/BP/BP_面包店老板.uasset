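; BP_面包店老板 (bakery owner) is an NPC that gives the player a quest to deliver a summer letter while avoiding dark clouds.
; On the player pawn's first overlap with its sphere, it opens WBP_对话界面 with hardcoded dialogue between 云小白 and 木小树 and ignores move and look input.
; It also adds the game HUD and coin counter then.
; The dialogue's close dispatcher (ED关闭) restores input.
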(event `self.Sphere.OnComponentBeginOverlap`
  (params (OverlappedComponent :type "PrimitiveComponent Object Reference") (OtherActor :type "Actor Object Reference") (OtherComp :type "PrimitiveComponent Object Reference") (OtherBodyIndex :type Integer) (bFromSweep :type Boolean) (SweepResult :type "HitResult Structure (by ref)"))
  (bind _returnvalue (`GameplayStatics.GetPlayerController` 0))
  (bind _returnvalue_2 (`GameplayStatics.GetPlayerController` 0))
  (if (== OtherActor (`GameplayStatics.GetPlayerPawn` 0))
    (`/Engine/EditorBlueprintResources/StandardMacros.DoOnce` false
      (:`Completed`
        (bind _returnvalue_3 (`|CreateWidget` "/Game/UI/WBP_对话界面.WBP_对话界面_C" null (`|MakeArray` (make `/Game/UI/S_对话内容` " 云小白" "我需要你帮我送一封夏日信件，但前方林间飘着扰乱方向的乌云，千万别碰到！") (make `/Game/UI/S_对话内容` "木小树" "那我要去哪里才能躲开这些乌云？") (make `/Game/UI/S_对话内容` "云小白" "远处那座蘑菇屋是中转站，只有平安走到那里，才能抵达阳光满满的夏日原野。") (make `/Game/UI/S_对话内容` "云小白" "你怀里的白云能护住你，一旦被乌云裹住，就会迷失，被迫回到这里重来。") (make `/Game/UI/S_对话内容` "木小树" "我一定会小心走到蘑菇屋，去往邮局！") (make `/Game/UI/S_对话内容` "云小白" "加油，我在这里等你平安归来！"))))
        (`UserWidget.AddToViewport` _returnvalue_3 0)
        (add `/Game/UI/WBP_对话界面.ED_关闭` _returnvalue_3 (delegate `完成对话`))
        (`Controller.SetIgnoreMoveInput` _returnvalue true)
        (`Controller.SetIgnoreLookInput` _returnvalue true)
        (bind _returnvalue_4 (`|CreateWidget` "/Game/ChallengeGame/UI/WB_GameHUD.WB_GameHUD_C" _returnvalue_2))
        (bind _returnvalue_5 (`|CreateWidget` "/Game/WBP_CoinCounter.WBP_CoinCounter_C" _returnvalue_2))
        (bind _output_get (set `self.Coin` _returnvalue_5))
        (`UserWidget.AddToViewport` _returnvalue_4 0)
        (`UserWidget.AddToViewport` _output_get 0)))))

(event `完成对话`
  (bind _returnvalue (`GameplayStatics.GetPlayerController` 0))
  (`Controller.SetIgnoreMoveInput` _returnvalue false)
  (`Controller.SetIgnoreLookInput` _returnvalue false))

(fn `UserConstructionScript`)