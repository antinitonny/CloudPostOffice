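; BP_小女孩 is a dialogue trigger actor that plays a one-time story conversation between 蘑小菇 and 木小树 at the mushroom waystation, pointing toward the summer plains.
; When the player pawn first enters its Sphere, a DoOnce creates WBP_对话界面 with hard-coded lines and blocks move and look input.
; The widget's ED关闭 dispatcher calls 完成对话 to restore input.
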(event `self.Sphere.OnComponentBeginOverlap`
  (params (OverlappedComponent :type "PrimitiveComponent Object Reference") (OtherActor :type "Actor Object Reference") (OtherComp :type "PrimitiveComponent Object Reference") (OtherBodyIndex :type Integer) (bFromSweep :type Boolean) (SweepResult :type "HitResult Structure (by ref)"))
  (bind _returnvalue (`GameplayStatics.GetPlayerController` 0))
  (if (== OtherActor (`GameplayStatics.GetPlayerPawn` 0))
    (`/Engine/EditorBlueprintResources/StandardMacros.DoOnce` false
      (:`Completed`
        (bind _returnvalue_2 (`|CreateWidget` "/Game/UI/WBP_对话界面.WBP_对话界面_C" null (`|MakeArray` (make `/Game/UI/S_对话内容` "蘑小菇" "你总算避开乌云平安到蘑菇中转屋啦，辛苦啦木小树！") (make `/Game/UI/S_对话内容` "木小树" "路上黑云总挡住路，还好有白云护着我，我的夏日信件还没送到云朵邮局。") (make `/Game/UI/S_对话内容` "蘑小菇" "这里只是中转站，邮局不在这片阴云林地，穿过屋后的通道就是夏日原野。") (make `/Game/UI/S_对话内容` "木小树" "夏日原野会很难走吗？") (make `/Game/UI/S_对话内容` "蘑小菇" "原野阳光充足没有乌云，但路上堆满石头、水坑和树枝障碍，得一路快跑躲开。") (make `/Game/UI/S_对话内容` "蘑小菇" "一直往前冲刺，原野最尽头就是云朵邮局，快把信件送过去吧！") (make `/Game/UI/S_对话内容` "木小树" "明白了，我这就出发赶往夏日原野！"))))
        (`UserWidget.AddToViewport` _returnvalue_2 0)
        (add `/Game/UI/WBP_对话界面.ED_关闭` _returnvalue_2 (delegate `完成对话`))
        (`Controller.SetIgnoreMoveInput` _returnvalue true)
        (`Controller.SetIgnoreLookInput` _returnvalue true)))))

(event `完成对话`
  (bind _returnvalue (`GameplayStatics.GetPlayerController` 0))
  (`Controller.SetIgnoreMoveInput` _returnvalue false)
  (`Controller.SetIgnoreLookInput` _returnvalue false))

(fn `UserConstructionScript`)