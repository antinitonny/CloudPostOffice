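; Rotating plank obstacle for the challenge game that catapults the third-person player on contact.
; A timeline spins the plank in yaw at a configurable rate, start offset and direction.
; Left and right trigger boxes apply a velocity-change impulse along their arrows and make the player jump.
; The construction script picks the long or short mesh, resizes and shifts the boxes for the short one, and rotates the arrows for reverse spin.
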(event `self.ReceiveBeginPlay`
  (bind _sm_plank_01 (`self.SM_Plank_01`))
  (bind _time_rotation (`self.Time rotation`))
  ;[1 1 1] Rotation, can control the forward and reverse rotation
  (`TimelineComponent.SetPlayRate` _time_rotation (`self.Rate Speed`))
  (`TimelineComponent.SetNewTime` _time_rotation (`self.Time Offset`))
  (bind (_direction _rota) (`Timeline|Time rotation`)
    (:`Update`
      (if (`self.Forward or Reverse`)
        (`SceneComponent.K2_SetRelativeRotation` _sm_plank_01 (`KismetMathLibrary.MakeRotator` 0.0 0.0 (* _rota -1.0)) false false)
        (else
          (`SceneComponent.K2_SetRelativeRotation` _sm_plank_01 (`KismetMathLibrary.MakeRotator` 0.0 0.0 _rota) false false))))))

(event `self.Box_L.OnComponentBeginOverlap`
  (params (OverlappedComponent :type "PrimitiveComponent Object Reference") (OtherActor :type "Actor Object Reference") (OtherComp :type "PrimitiveComponent Object Reference") (OtherBodyIndex :type Integer) (bFromSweep :type Boolean) (SweepResult :type "HitResult Structure (by ref)"))
  ;[1 1 1] Catapult the player in the direction of the arrow
  (bind _asbp_third_person (cast `/Game/ChallengeGame/Demo/ThirdPerson/Blueprints/BP_ThirdPerson` OtherActor))
  (`CharacterMovementComponent.AddImpulse` (`Character.CharacterMovement` _asbp_third_person) (* (`SceneComponent.GetForwardVector` (`self.Arrow_L`)) (`self.Repel Force`)) true)
  (`Character.Jump` _asbp_third_person))

(event `self.Box_R.OnComponentBeginOverlap`
  (params (OverlappedComponent :type "PrimitiveComponent Object Reference") (OtherActor :type "Actor Object Reference") (OtherComp :type "PrimitiveComponent Object Reference") (OtherBodyIndex :type Integer) (bFromSweep :type Boolean) (SweepResult :type "HitResult Structure (by ref)"))
  ;[1 1 1] Catapult the player in the direction of the arrow
  (bind _asbp_third_person (cast `/Game/ChallengeGame/Demo/ThirdPerson/Blueprints/BP_ThirdPerson` OtherActor))
  (`CharacterMovementComponent.AddImpulse` (`Character.CharacterMovement` _asbp_third_person) (* (`SceneComponent.GetForwardVector` (`self.Arrow_R`)) (`self.Repel Force`)) true)
  (`Character.Jump` _asbp_third_person))

(fn `UserConstructionScript`
  (bind _box_l (`self.Box_L`))
  (bind _arrow_r (`self.Arrow_R`))
  (bind _sm_plank_01 (`self.SM_Plank_01`))
  (bind _box_r (`self.Box_R`))
  (bind _returnvalue (`SceneComponent.GetRelativeTransform` _box_r))
  (bind _returnvalue_2 (`SceneComponent.GetRelativeTransform` _box_l))
  (if (`self.Long or Short`)
    (`StaticMeshComponent.SetStaticMesh` _sm_plank_01 (`self.LongMesh`))
    (else
      (`StaticMeshComponent.SetStaticMesh` _sm_plank_01 (`self.ShortMesh`))
      (`SceneComponent.K2_SetRelativeTransform` _box_r (`KismetMathLibrary.MakeTransform` (`KismetMathLibrary.MakeVector` (- (.x (.location _returnvalue)) -170.0) (.y (.location _returnvalue)) (.z (.location _returnvalue))) (.rotation _returnvalue) (`KismetMathLibrary.MakeVector` (/ (.x (.scale _returnvalue)) 2.5) (.y (.scale _returnvalue)) (.z (.scale _returnvalue)))) false false)
      (`SceneComponent.K2_SetRelativeTransform` _box_l (`KismetMathLibrary.MakeTransform` (`KismetMathLibrary.MakeVector` (- (.x (.location _returnvalue_2)) 170.0) (.y (.location _returnvalue_2)) (.z (.location _returnvalue_2))) (.rotation _returnvalue_2) (`KismetMathLibrary.MakeVector` (/ (.x (.scale _returnvalue_2)) 2.5) (.y (.scale _returnvalue_2)) (.z (.scale _returnvalue_2)))) false false)))
  ;[1 1 1] Change arrow direction
  (if (`self.Forward or Reverse`)
    (`SceneComponent.K2_AddRelativeRotation` _arrow_r (struct :`Yaw` 180.0) false false)
    (`SceneComponent.K2_AddRelativeRotation` (`self.Arrow_L`) (struct :`Yaw` 180.0) false false)
    (else
      (`SceneComponent.K2_AddRelativeRotation` :`self` _arrow_r)
      (`SceneComponent.K2_AddRelativeRotation` :`self` (`self.Arrow_L`)))))