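; BP_SpherePendulum is a swinging sphere hazard that kills the player character on contact.
; On BeginPlay it starts a timeline with configurable play rate and start time, whose track, scaled by Range, sets the relative pitch of SMSphere.
; The Inversion flag negates that pitch to mirror the swing.
; An overlap on the Sphere component casts the other actor to BP_ThirdPerson and calls its Death function.
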(event `self.ReceiveTick`
  (params (DeltaSeconds :type "Float (single-precision)")))

(event `self.ReceiveBeginPlay`
  (bind _sm_sphere (`self.SM_Sphere`))
  (bind _time_line (`self.Time line`))
  (`TimelineComponent.SetPlayRate` _time_line (`self.New Rate`))
  (`TimelineComponent.SetNewTime` _time_line (`self.New Time`))
  (bind (_direction `_新建轨道_0`) (`Timeline|Time line`)
    (:`Update`
      (if (`self.Inversion`)
        (bind _returnvalue (* `_新建轨道_0` (`self.Range`)))
        (`SceneComponent.K2_SetRelativeRotation` _sm_sphere (`KismetMathLibrary.MakeRotator` 0.0 (* _returnvalue -1.0)) false false)
        (else
          (`SceneComponent.K2_SetRelativeRotation` _sm_sphere (`KismetMathLibrary.MakeRotator` 0.0 _returnvalue) false false))))))

(event `self.Sphere.OnComponentBeginOverlap`
  (params (OverlappedComponent :type "PrimitiveComponent Object Reference") (OtherActor :type "Actor Object Reference") (OtherComp :type "PrimitiveComponent Object Reference") (OtherBodyIndex :type Integer) (bFromSweep :type Boolean) (SweepResult :type "HitResult Structure (by ref)"))
  (bind _asbp_third_person (cast `/Game/ChallengeGame/Demo/ThirdPerson/Blueprints/BP_ThirdPerson` OtherActor))
  (`/Game/ChallengeGame/Demo/ThirdPerson/Blueprints/BP_ThirdPerson.Death` _asbp_third_person))

(fn `UserConstructionScript`)