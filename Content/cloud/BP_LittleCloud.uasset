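; BP_LittleCloud is a small cloud actor that follows the player character.
; Each Tick eases it with VInterpTo toward a world-space offset from player 0, with CloudSide scaling the sideways (Y) offset.
; SetCloudDark switches its three cloud meshes between the normal and dark cloud materials.
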(event `self.ReceiveTick`
  (params (DeltaSeconds :type "Float (single-precision)"))
  (`self.K2_SetActorLocation` (`KismetMathLibrary.VInterpTo` (`self.K2_GetActorLocation`) (+ (`self.K2_GetActorLocation` (`GameplayStatics.GetPlayerCharacter` 0)) (`KismetMathLibrary.MakeVector` 100.0 (* (`self.CloudSide`) 100.0) 50.0)) DeltaSeconds 5.0)))

(fn `SetCloudDark`
  (params (bDark :type Boolean))
  (if bDark
    (`|ExecutionSequence`
      (:`then_0`
        (`PrimitiveComponent.SetMaterial` (`self.CloudMesh`) 0 "/Game/cloud/M_Cloud_Dark.M_Cloud_Dark"))
      (:`then_1`
        (`PrimitiveComponent.SetMaterial` (`self.CloudMesh2`) 0 "/Game/cloud/M_Cloud_Dark.M_Cloud_Dark"))
      (:`then_2`
        (`PrimitiveComponent.SetMaterial` (`self.CloudMesh1`) 0 "/Game/cloud/M_Cloud_Dark.M_Cloud_Dark")))
    (else
      (`|ExecutionSequence`
        (:`then_0`
          (`PrimitiveComponent.SetMaterial` (`self.CloudMesh`) 0 "/Game/cloud/M_Cloud.M_Cloud"))
        (:`then_1`
          (`PrimitiveComponent.SetMaterial` (`self.CloudMesh2`) 0 "/Game/cloud/M_Cloud.M_Cloud"))
        (:`then_2`
          (`PrimitiveComponent.SetMaterial` (`self.CloudMesh1`) 0 "/Game/cloud/M_Cloud.M_Cloud"))))))

(fn `UserConstructionScript`)