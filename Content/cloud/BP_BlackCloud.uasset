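; BP_BlackCloud is a constantly spinning hazard cloud that resets the player and BP_LittleCloud to the world origin.
; Any overlap with its Box darkens the BP_LittleCloud found by class lookup and waits briefly.
; It then moves player character 0 and the little cloud to the origin and clears the dark state, without checking which actor triggered the overlap.
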(event `self.ReceiveTick`
  (params (DeltaSeconds :type "Float (single-precision)"))
  (`self.K2_AddActorLocalRotation` (struct :`Yaw` 1.0)))

(event `self.Box.OnComponentBeginOverlap`
  (params (OverlappedComponent :type "PrimitiveComponent Object Reference") (OtherActor :type "Actor Object Reference") (OtherComp :type "PrimitiveComponent Object Reference") (OtherBodyIndex :type Integer) (bFromSweep :type Boolean) (SweepResult :type "HitResult Structure (by ref)"))
  (bind _returnvalue (`GameplayStatics.GetActorOfClass` "/Game/cloud/BP_LittleCloud.BP_LittleCloud_C"))
  (`/Game/cloud/BP_LittleCloud.SetCloudDark` _returnvalue true)
  (`KismetSystemLibrary.Delay` 1.0)
  (`|ExecutionSequence`
    (:`then_0`
      (`self.K2_SetActorLocation` (`GameplayStatics.GetPlayerCharacter` 0) (0.0 0.0 0.0) false false))
    (:`then_1`
      (bind _returnvalue_2 (`GameplayStatics.GetActorOfClass` "/Game/cloud/BP_LittleCloud.BP_LittleCloud_C"))))
  (`self.K2_SetActorLocation` _returnvalue_2 (0.0 0.0 0.0) false false)
  (bind _returnvalue_3 (`GameplayStatics.GetActorOfClass` "/Game/cloud/BP_LittleCloud.BP_LittleCloud_C"))
  (`/Game/cloud/BP_LittleCloud.SetCloudDark` _returnvalue_3 false))

(fn `UserConstructionScript`)